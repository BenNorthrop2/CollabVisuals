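; Test Blueprint for the TechFaceCrawler enemy, trying out physics-blended animation and a laser effect.
; BeginPlay simulates bodies below "Body", applies a strengthened "Main" physical animation profile at partial blend weight, disables laser rendering and starts a looping timer.
; Fire activates the Niagara laser toward the static mesh's location, then deactivates it after a short delay.
; The SetSkeletalMeshComponent call that would bind physical animation to the mesh is disconnected.
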(event Custom|Fire
  (Components|Activation|Activate (Variables|Default|GetNS_Laser) false)
  (Class|NiagaraComponent|SetVariablePosition (Variables|Default|GetNS_Laser) "Beam End" (Transformation|GetWorldLocation (Variables|Default|GetStaticMesh)))
  (Utilities|FlowControl|Delay 1.0)
  (CallFunction|StopFire))

(event Custom|StopFire
  (Components|Activation|Deactivate (Variables|Default|GetNS_Laser)))

(event EventBeginPlay
  (bind _physicalanimation (Variables|Default|GetPhysicalAnimation))
  (Class|SkeletalMeshComponent|SetAllBodiesBelowSimulatePhysics (Variables|Default|GetSkeletalMesh) (Utilities|Name|MakeLiteralName "Body") true false)
  (Class|PhysicalAnimationComponent|ApplyPhysicalAnimationProfileBelow _physicalanimation "Body" "Main" true true)
  (Class|SkeletalMeshComponent|SetAllBodiesPhysicsBlendWeight (Variables|Default|GetSkeletalMesh) 0.4 false)
  (Class|PhysicalAnimationComponent|SetStrengthMultiplyer _physicalanimation 3.0)
  (Class|NiagaraComponent|SetRenderingEnabled (Variables|Default|GetNS_Laser) false)
  (Utilities|Time|SetTimerbyEvent (EventDispatchers|CreateEvent :!event Custom|Fire) 5.0 true))

(fn ConstructionScript)