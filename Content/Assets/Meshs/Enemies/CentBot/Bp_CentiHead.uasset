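; Head actor of the CentBot centipede enemy that spawns a chain of Bp_CentiBody segments and drags them behind it.
; BeginPlay lines the segments up along the negative right axis into BodyActors.
; Each Tick sends scaled mesh velocity to the anim instance, then adjusts every segment against its predecessor, the first against the head mesh.
; Segments turn and interpolate closer beyond ChaseDistance, or toward an offset behind the leader inside BackAwayDistance.
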(event Custom|UpdateChasePosition
  (bind _skeletalmesh (Variables|Default|GetSkeletalMesh))
  (bind _chasedistance (Variables|Default|GetChaseDistance))
  ;[1 1 1] Comment
  (for (_array_element _array_index) (Variables|Default|GetBodyActors)
    (Utilities|IsValid _array_element
      (:Is%20Valid
        (if (== _array_index 0)
          (if (> (Math|Vector|Distance(Vector) (.Location (Math|Transform|BreakTransform (Transformation|GetActorTransform (Utilities|Array|Get(acopy) (Variables|Default|GetBodyActors))))) (.Location (Math|Transform|BreakTransform (Transformation|GetWorldTransform (Variables|Default|GetSkeletalMesh))))) _chasedistance)
            (Transformation|SetActorTransform (Utilities|Array|Get(acopy) (Variables|Default|GetBodyActors) _array_index) (Class|KismetMathLibrary|TInterpto (Transformation|GetActorTransform (Utilities|Array|Get(acopy) (Variables|Default|GetBodyActors) _array_index)) (Class|KismetAnimationLibrary|Lookat (Transformation|GetActorTransform (Utilities|Array|Get(acopy) (Variables|Default|GetBodyActors) _array_index)) (Transformation|GetWorldLocation _skeletalmesh) "0.000000,1.000000,0.000000" true "0.000000,0.000000,1.000000" 0.0) (Utilities|Time|GetWorldDeltaSeconds) (Variables|Default|GetFollowSpeed)) (Variables|Default|GetSweep))
            (Transformation|SetActorTransform (Utilities|Array|Get(acopy) (Variables|Default|GetBodyActors) _array_index) (Class|KismetMathLibrary|TInterpto (Transformation|GetActorTransform (Utilities|Array|Get(acopy) (Variables|Default|GetBodyActors) _array_index)) (Transformation|GetWorldTransform _skeletalmesh) (Utilities|Time|GetWorldDeltaSeconds) (Variables|Default|GetFollowSpeed)) (Variables|Default|GetSweep)))
          (elif (> (Math|Vector|Distance(Vector) (.Location (Math|Transform|BreakTransform (Transformation|GetActorTransform (Utilities|Array|Get(acopy) (Variables|Default|GetBodyActors) _array_index)))) (.Location (Math|Transform|BreakTransform (Transformation|GetActorTransform (Utilities|Array|Get(acopy) (Variables|Default|GetBodyActors) (+ _array_index -1)))))) _chasedistance)
            (Transformation|SetActorTransform (Utilities|Array|Get(acopy) (Variables|Default|GetBodyActors) _array_index) (Class|KismetMathLibrary|TInterpto (Transformation|GetActorTransform (Utilities|Array|Get(acopy) (Variables|Default|GetBodyActors) _array_index)) (Class|KismetAnimationLibrary|Lookat (Transformation|GetActorTransform (Utilities|Array|Get(acopy) (Variables|Default|GetBodyActors) _array_index)) (.Location (Math|Transform|BreakTransform (Transformation|GetActorTransform (Utilities|Array|Get(acopy) (Variables|Default|GetBodyActors) (+ _array_index -1))))) "0.000000,1.000000,0.000000" true "0.000000,0.000000,1.000000" 0.0) (Utilities|Time|GetWorldDeltaSeconds) (Variables|Default|GetFollowSpeed)) (Variables|Default|GetSweep))
            (Transformation|SetActorTransform (Utilities|Array|Get(acopy) (Variables|Default|GetBodyActors) _array_index) (Class|KismetMathLibrary|TInterpto (Transformation|GetActorTransform (Utilities|Array|Get(acopy) (Variables|Default|GetBodyActors) _array_index)) (Transformation|GetActorTransform (Utilities|Array|Get(acopy) (Variables|Default|GetBodyActors) (+ _array_index -1))) (Utilities|Time|GetWorldDeltaSeconds) (Variables|Default|GetFollowSpeed)) (Variables|Default|GetSweep))))))))

(event Custom|UpdateBackawayPositoin
  (bind _skeletalmesh (Variables|Default|GetSkeletalMesh))
  (bind _backawaydistance (Variables|Default|GetBackAwayDistance))
  ;[1 1 1] Comment
  (for (_array_element _array_index) (Variables|Default|GetBodyActors)
    (Utilities|IsValid _array_element
      (:Is%20Valid
        (if (== _array_index 0)
          (if (< (Math|Vector|Distance(Vector) (.Location (Math|Transform|BreakTransform (Transformation|GetActorTransform (Utilities|Array|Get(acopy) (Variables|Default|GetBodyActors))))) (.Location (Math|Transform|BreakTransform (Transformation|GetWorldTransform (Variables|Default|GetSkeletalMesh))))) _backawaydistance)
            (Transformation|SetActorTransform (Utilities|Array|Get(acopy) (Variables|Default|GetBodyActors) _array_index) (Class|KismetMathLibrary|TInterpto (Transformation|GetActorTransform (Utilities|Array|Get(acopy) (Variables|Default|GetBodyActors) _array_index)) (Class|KismetAnimationLibrary|Lookat (Transformation|GetActorTransform (Utilities|Array|Get(acopy) (Variables|Default|GetBodyActors) _array_index)) (Transformation|GetWorldLocation _skeletalmesh) "0.000000,1.000000,0.000000" true "0.000000,0.000000,1.000000" 0.0) (Utilities|Time|GetWorldDeltaSeconds) (Variables|Default|GetFollowSpeed)) (Variables|Default|GetSweep))
            (Transformation|SetActorTransform (Utilities|Array|Get(acopy) (Variables|Default|GetBodyActors) _array_index) (Class|KismetMathLibrary|TInterpto (Transformation|GetActorTransform (Utilities|Array|Get(acopy) (Variables|Default|GetBodyActors) _array_index)) (Math|Transform|MakeTransform (+ (* (Math|Vector|GetRightVector _skeletalmesh) (Math|Float|MakeLiteralFloat -5e+01)) (.Location (Math|Transform|BreakTransform (Transformation|GetWorldTransform _skeletalmesh)))) (.Rotation (Math|Transform|BreakTransform (Transformation|GetActorTransform (Utilities|Array|Get(acopy) (Variables|Default|GetBodyActors) _array_index)))) (.Scale (Math|Transform|BreakTransform (Transformation|GetActorTransform (Utilities|Array|Get(acopy) (Variables|Default|GetBodyActors) _array_index))))) (Utilities|Time|GetWorldDeltaSeconds) (Variables|Default|GetFollowSpeed)) (Variables|Default|GetSweep)))
          (elif (< (Math|Vector|Distance(Vector) (.Location (Math|Transform|BreakTransform (Transformation|GetActorTransform (Utilities|Array|Get(acopy) (Variables|Default|GetBodyActors) (+ _array_index -1))))) (.Location (Math|Transform|BreakTransform (Transformation|GetActorTransform (Utilities|Array|Get(acopy) (Variables|Default|GetBodyActors) _array_index))))) _backawaydistance)
            (Transformation|SetActorTransform (Utilities|Array|Get(acopy) (Variables|Default|GetBodyActors) _array_index) (Class|KismetMathLibrary|TInterpto (Transformation|GetActorTransform (Utilities|Array|Get(acopy) (Variables|Default|GetBodyActors) _array_index)) (Class|KismetAnimationLibrary|Lookat (Transformation|GetActorTransform (Utilities|Array|Get(acopy) (Variables|Default|GetBodyActors) _array_index)) (.Location (Math|Transform|BreakTransform (Transformation|GetActorTransform (Utilities|Array|Get(acopy) (Variables|Default|GetBodyActors) (+ _array_index -1))))) "0.000000,1.000000,0.000000" true "0.000000,0.000000,1.000000" 0.0) (Utilities|Time|GetWorldDeltaSeconds) (Variables|Default|GetFollowSpeed)) (Variables|Default|GetSweep))
            (Transformation|SetActorTransform (Utilities|Array|Get(acopy) (Variables|Default|GetBodyActors) _array_index) (Class|KismetMathLibrary|TInterpto (Transformation|GetActorTransform (Utilities|Array|Get(acopy) (Variables|Default|GetBodyActors) _array_index)) (Math|Transform|MakeTransform (+ (.Location (Math|Transform|BreakTransform (Transformation|GetActorTransform (Utilities|Array|Get(acopy) (Variables|Default|GetBodyActors) (+ _array_index -1))))) (* (Transformation|GetActorRightVector (Utilities|Array|Get(acopy) (Variables|Default|GetBodyActors) (+ _array_index -1))) (Math|Float|MakeLiteralFloat -5e+01))) (.Rotation (Math|Transform|BreakTransform (Transformation|GetActorTransform (Utilities|Array|Get(acopy) (Variables|Default|GetBodyActors) _array_index)))) (.Scale (Math|Transform|BreakTransform (Transformation|GetActorTransform (Utilities|Array|Get(acopy) (Variables|Default|GetBodyActors) _array_index))))) (Utilities|Time|GetWorldDeltaSeconds) (Variables|Default|GetFollowSpeed)) (Variables|Default|GetSweep))))))))

(event EventTick
  (params (DeltaSeconds :type Float%20%28single-precision%29))
  ;[1 1 1] Comment
  (Class|IFANIMEnemy|VelocityPass(Message) (Components|SkeletalMesh|GetAnimInstance (Variables|Default|GetSkeletalMesh)) (* (Transformation|GetComponentVelocity (Variables|Default|GetSkeletalMesh)) (Math|Float|MakeLiteralFloat 15.0)))
  (CallFunction|UpdateChasePosition)
  (CallFunction|UpdateBackawayPositoin))

(event EventBeginPlay
  (bind _self self)
  (bind _returnvalue (Transformation|GetActorTransform _self))
  (bind (_location _rotation _scale) (Math|Transform|BreakTransform _returnvalue))
  ;[1 1 1] Comment
  (bind _index (Utilities|FlowControl|ForLoopwithBreak 0 (Variables|Default|GetBodyCount))
    (:LoopBody
      (bind _returnvalue_2 (Game|SpawnActorfromClass "/Game/Assets/Meshs/Enemies/CentBot/Bp_CentiBody.Bp_CentiBody_C" (Math|Transform|MakeTransform (+ (* (Transformation|GetActorRightVector _self) (* (+ _index 1) (Math|Float|MakeLiteralFloat -25.0))) _location) _rotation _scale) "Undefined" "MultiplyWithRoot" 0 0))
      (Utilities|Array|Add (Variables|Default|GetBodyActors) _returnvalue_2))))

(fn ConstructionScript)