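; Body segment actor of the CentBot enemy that keeps itself at the height of the ground beneath it.
; Each Tick, a small vertical sphere trace against WorldStatic objects runs from above to below the actor.
; On a hit, the actor eases its Z toward the impact point with a swept VInterpTo move, keeping X and Y.
; Slope-tilt rotation math from the hit normal is present but unconnected.
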(event EventTick
  (params (DeltaSeconds :type Float%20%28single-precision%29))
  (bind _returnvalue (Transformation|GetActorLocation))
  (bind _returnvalue_2 (Transformation|GetActorLocation))
  (bind (_x _y) (Math|Vector|BreakVector _returnvalue_2))
  (bind _z (Math|Vector|BreakVector _returnvalue_2))
  (Utilities|IsValid self
    (:Is%20Valid
      (bind (_outhit _returnvalue_3) (Collision|SphereTraceForObjects (Math|Vector|MakeVector _x _y (+ _z 1.5e+02)) (Math|Vector|MakeVector _x _y (+ _z -8e+01)) 7.0 (Utilities|Array|MakeArray "ObjectTypeQuery1") false 0 "None" true "(R=1.000000,G=0.000000,B=0.000000,A=1.000000)" "(R=0.000000,G=1.000000,B=0.000000,A=1.000000)" 1.0))
      (Transformation|SetActorLocation (Math|Interpolation|VInterpTo _returnvalue (Math|Vector|SelectVector (Math|Vector|MakeVector _x _y (.z (.ImpactPoint (Collision|BreakHitResult _outhit)))) _returnvalue _returnvalue_3) (Utilities|Time|GetWorldDeltaSeconds) 9.0) true false))))

(fn ConstructionScript)